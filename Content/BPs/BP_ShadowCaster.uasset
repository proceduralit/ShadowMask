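; Shadow caster actor that aims a directional light and a scene capture rig from sun azimuth and altitude, with the capture showing only this actor.
; UpdateTransformation, run at construction and BeginPlay, publishes the capture's location and axes to MPC_TransformationData and its matrix to Niagara as LightMatrix.
; RT_FadeShadow is cleared at BeginPlay, then redrawn with M_FadeShadow through a short Tick delay that throttles updates.
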(event `self.ReceiveBeginPlay`
  (`KismetRenderingLibrary.ClearRenderTarget2D` "/Game/Mats/RT_FadeShadow.RT_FadeShadow")
  (`self.UpdateTransformation`))

(event `self.ReceiveTick`
  (params (DeltaSeconds :type "Float (single-precision)"))
  (`KismetSystemLibrary.Delay` 0.05)
  (`KismetRenderingLibrary.DrawMaterialToRenderTarget` "/Game/Mats/RT_FadeShadow.RT_FadeShadow" "/Game/Mats/M_FadeShadow.M_FadeShadow"))

(fn `UpdateTransformation`
  (bind _sun_azimuth (`self.Sun Azimuth`))
  (bind _returnvalue (`SceneComponent.K2_GetComponentToWorld` (`self.SceneCaptureComponent2D`)))
  (bind _returnvalue_2 (* (`self.Sun Altitude`) -1.0))
  (bind _rotation (.rotation _returnvalue))
  (`SceneComponent.K2_SetRelativeRotation` (`self.DirectionalLight`) (`KismetMathLibrary.MakeRotator` 0.0 _returnvalue_2 _sun_azimuth) false false)
  (`SceneComponent.K2_SetRelativeRotation` (`self.Scene`) (`KismetMathLibrary.MakeRotator` 0.0 _returnvalue_2 _sun_azimuth) false false)
  (`KismetMaterialLibrary.SetVectorParameterValue` "/Game/Mats/MPC_TransformationData.MPC_TransformationData" "Location" (`KismetMathLibrary.Conv_VectorToLinearColor` (.location _returnvalue)))
  (`KismetMaterialLibrary.SetVectorParameterValue` "/Game/Mats/MPC_TransformationData.MPC_TransformationData" "Up" (`KismetMathLibrary.Conv_VectorToLinearColor` (`KismetMathLibrary.GetUpVector` _rotation)))
  (`KismetMaterialLibrary.SetVectorParameterValue` "/Game/Mats/MPC_TransformationData.MPC_TransformationData" "Forward" (`KismetMathLibrary.Conv_VectorToLinearColor` (`KismetMathLibrary.GetForwardVector` _rotation)))
  (`KismetMaterialLibrary.SetVectorParameterValue` "/Game/Mats/MPC_TransformationData.MPC_TransformationData" "Right" (`KismetMathLibrary.Conv_VectorToLinearColor` (`KismetMathLibrary.GetRightVector` _rotation)))
  (`NiagaraComponent.SetVariableMatrix` (`self.Niagara`) "LightMatrix" (`KismetMathLibrary.Conv_TransformToMatrix` _returnvalue)))

(fn `UserConstructionScript`
  (`KismetArrayLibrary.Array_Add` (`SceneCaptureComponent.ShowOnlyActors` (`self.SceneCaptureComponent2D`)) self)
  (`self.UpdateTransformation`))